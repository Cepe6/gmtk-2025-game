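; GM_Platformer is a platformer game mode that spawns players and tracks whether all have reached a finish.
; On BeginPlay it spawns a BP_Player at each PlayerStart, stores it in ActiveActors and possesses each with player controller 0, leaving the last possessed.
; It binds to every BP_Finish touch dispatcher.
; Each dispatch checks every active actor's IsTouchingFinish flag and only prints the combined result.
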(event Custom|OnActorFinishStateUpdate
  (bind _actorsonfinish (CallFunction|AreAllActorsonFinish))
  (Development|PrintString (Utilities|String|ToString(Boolean) _actorsonfinish)))

(event EventBeginPlay
  (CallFunction|InitialiseGame)
  (bind _outactors (Actor|GetAllActorsOfClass "/Game/Blueprints/BP_Finish.BP_Finish_C"))
  (for _array_element _outactors
    (EventDispatchers|BindEventtoFinishTouchDispatcher _array_element (delegate Custom|OnActorFinishStateUpdate))))

(fn ConstructionScript)

(fn AreAllActorsonFinish
  (Variables|Default|SetActorsOnFinish true)
  (for _array_element (Variables|Default|GetActiveActors)
    (Variables|Default|SetActorsOnFinish (and (Variables|Default|GetActorsOnFinish) (Variables|/Game/Blueprints/BP_Player.BP_Player_C|GetIs%20Touching%20Finish _array_element))))
  (return (Variables|Default|GetActorsOnFinish)))

(fn InitialiseGame
  (bind _outactors (Actor|GetAllActorsOfClass "/Script/Engine.PlayerStart"))
  (for _array_element _outactors
    (bind _returnvalue (Game|SpawnActorfromClass "/Game/Blueprints/BP_Player.BP_Player_C" (Transformation|GetActorTransform _array_element) "Undefined" "MultiplyWithRoot" 0 0))
    (Utilities|Array|Add (Variables|Default|GetActiveActors) _returnvalue)
    (Pawn|Possess (Game|GetPlayerController 0) _returnvalue)))